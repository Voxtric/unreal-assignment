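; Grunt enemy AI that roams, patrols between two points, or chases and attacks the player, with a floating health bar.
; DecideState dispatches on AIState to AI MoveTo events, which call it again after successful moves and waits.
; Pawn sensing switches the state to Chase on first player sighting, effective at the next DecideState.
; Tick updates the camera-facing health widget and turns the grunt toward the player while chasing.
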(event `self.ReceiveBeginPlay`
  (`self.DecideState`))

(event `self.ReceiveTick`
  (params (DeltaSeconds :type "Float (single-precision)"))
  (bind _asenemy_health (cast `/Game/UI/Enemy_Health` (`WidgetComponent.GetUserWidgetObject` (`self.Health`))))
  (`ProgressBar.SetPercent` (`/Game/UI/Enemy_Health.ProgressBar_22` _asenemy_health) (/ (`self.TotalHealth`) 100.0))
  (`SceneComponent.K2_SetWorldRotation` (`self.Health`) (`KismetMathLibrary.FindLookAtRotation` (`SceneComponent.K2_GetComponentLocation` (`self.Health`)) (`self.K2_GetActorLocation` (`GameplayStatics.GetPlayerCameraManager` 0))) false false)
  (switch `/Game/AI_Data/EAIState` (`self.AIState`)
    (:`NewEnumerator2`
      (`self.K2_SetActorRotation` (`KismetMathLibrary.FindLookAtRotation` (`self.K2_GetActorLocation`) (`self.K2_GetActorLocation` (`GameplayStatics.GetPlayerCharacter` 0)))))))

(event `Roam`
  (`|AIMoveTo` self (`NavigationSystem.GetRandomPointInNavigableRadius` (`self.K2_GetActorLocation`) 500.0)
    (:`OnSuccess`
      (`KismetSystemLibrary.Delay` (`KismetMathLibrary.RandomFloatInRange` 0.0 0.5))
      (`self.DecideState`))))

(event `ChasePlayer`
  (params (PlayerToChase :type "/Game/Player/ThirdPersonCharacter Object Reference"))
  (`|AIMoveTo` self (0.0 0.0 0.0) PlayerToChase 5.0
    (:`OnSuccess`
      (`self.OnPerformAttack`)
      (`KismetSystemLibrary.Delay` 5.0)
      (`self.DecideState`))))

(event `Patrol`
  (`|AIMoveTo` self (0.0 0.0 0.0) (`self.Patrol1`) 5.0
    (:`OnSuccess`
      (`KismetSystemLibrary.Delay` (`self.PatrolWait`))
      (`|AIMoveTo` self (0.0 0.0 0.0) (`self.Patrol2`)
        (:`OnSuccess`
          (`KismetSystemLibrary.Delay` (`self.PatrolWait`))
          (`self.DecideState`))))))

(event `self.PawnSensor.OnSeePawn`
  (params (Pawn :type "Pawn Object Reference"))
  ;[1 1 1] Chase player when we see them
  (if (not (`self.SeenPlayer`))
    (cast `/Game/Player/ThirdPersonCharacter` Pawn)
    (set `self.AIState` "NewEnumerator2")
    (set `self.SeenPlayer` true)))

(fn `DecideState`
  (bind _asthird_person_character (cast `/Game/Player/ThirdPersonCharacter` (`GameplayStatics.GetPlayerCharacter` 0)))
  (switch `/Game/AI_Data/EAIState` (`self.AIState`)
    (:`NewEnumerator1`
      (`self.Roam`))
    (:`NewEnumerator2`
      (`self.ChasePlayer` _asthird_person_character))
    (:`NewEnumerator3`
      (`self.Patrol`))))

(fn `UserConstructionScript`)
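; BP_Pickup is an interactable item that the player collects into their inventory.
; Interact adds the item by ID through BP_GameplayController, runs a placeholder sound step with a debug reminder, then destroys the actor.
; Destroyed passes PickupPopUp to the player ThirdPersonCharacter's PickupEvent.
; An unconnected leftover branch would add ScoreTotal to an AssignmentCharacter's score, but it never runs.
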(event `self.Interact`
  (params (Controller :type "PlayerController Object Reference"))
  (`GameplayController.AddItemToInventoryByID` (cast `/Game/Blueprints/BP_GameplayController` Controller :!pure true) (`self.ItemID`))
  (`KismetSystemLibrary.PrintString` "Needs Sound effect in blueprint of BP_Pickup")
  (`GameplayStatics.PlaySound2D` null)
  (`self.K2_DestroyActor`))

(event `self.ReceiveDestroyed`
  (bind _asthird_person_character (cast `/Game/Player/ThirdPersonCharacter` (`GameplayStatics.GetPlayerCharacter` 0)))
  (`/Game/Player/ThirdPersonCharacter.Pickup_Event` _asthird_person_character (`self.PickupPopUp`)))

(fn `UserConstructionScript`)
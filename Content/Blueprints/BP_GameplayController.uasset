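; Player controller that toggles the inventory screen for the controlled third-person character.
; On the Open_Inventory press, if the character is controllable, it lazily creates a WB_Inventory widget and reuses it, adding it to or removing it from the viewport.
; Move input is ignored while the inventory is open, and opening it sets game-only input mode.
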(event `InputAction|Open_Inventory`
  (params (Key :type "Key Structure" :default "AnyKey"))
  (bind _inventoryopen (`self.InventoryOpen`))
  (bind _inventory_widget (`self.Inventory_Widget`))
  ;[1 1 1] Open the players inventory when the input action is received
  (:`Pressed`
    (bind _asthird_person_character (cast `/Game/Player/ThirdPersonCharacter` (`self.K2_GetPawn`)))
    (if (`AssignmentCharacter.IsControlable` _asthird_person_character)
      (`/Engine/EditorBlueprintResources/StandardMacros.IsValid` (`self.Inventory_Widget`) :!label _label
        (:`Is Valid`
          (`self.SetIgnoreMoveInput` (`GameplayStatics.GetPlayerController` 0) (not _inventoryopen))
          (if _inventoryopen
            (`Widget.RemoveFromParent` _inventory_widget)
            (set `self.InventoryOpen` false)
            (else
              (`UserWidget.AddToViewport` _inventory_widget 0)
              (set `self.InventoryOpen` true)
              (`WidgetBlueprintLibrary.SetInputMode_GameOnly` (`GameplayStatics.GetPlayerController` 0)))))
        (:`Is Not Valid`
          (bind _returnvalue (`|CreateWidget` "/Game/UI/WB_Inventory.WB_Inventory_C"))
          (set `self.Inventory_Widget` _returnvalue)
          (goto _label))))))

(fn `UserConstructionScript`)
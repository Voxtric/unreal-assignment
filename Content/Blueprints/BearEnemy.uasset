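; Bear enemy AI character with a floating health bar that updates and turns toward the camera each tick.
; DecideState only handles Patrol, which loops AIMoveTo between two points with pauses.
; Roam, ChasePlayer with attack, and an alternate patrol event exist but are not called here.
; Tick faces the player in Chase state, but pawn sensing only casts the seen pawn; the code setting Chase is disconnected.
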(event `self.ReceiveBeginPlay`
  (`self.DecideState`))

(event `self.ReceiveTick`
  (params (DeltaSeconds :type "Float (single-precision)"))
  (bind _asenemy_health (cast `/Game/UI/Enemy_Health` (`WidgetComponent.GetUserWidgetObject` (`self.Widget`))))
  (`ProgressBar.SetPercent` (`/Game/UI/Enemy_Health.ProgressBar_22` _asenemy_health) (/ (`self.TotalHealth`) 100.0))
  (`SceneComponent.K2_SetWorldRotation` (`self.Widget`) (`KismetMathLibrary.FindLookAtRotation` (`SceneComponent.K2_GetComponentLocation` (`self.Widget`)) (`self.K2_GetActorLocation` (`GameplayStatics.GetPlayerCameraManager` 0))) false false)
  (switch `/Game/AI_Data/EAIState` (`self.AIState`)
    (:`NewEnumerator2`
      (`self.K2_SetActorRotation` (`KismetMathLibrary.FindLookAtRotation` (`self.K2_GetActorLocation`) (`self.K2_GetActorLocation` (`GameplayStatics.GetPlayerCharacter` 0)))))))

(event `Patrol`
  (`|AIMoveTo` self (0.0 0.0 0.0) (`self.Patrol1`)
    (:`OnSuccess`
      (`KismetSystemLibrary.Delay` 5.0)
      (`|AIMoveTo` self (0.0 0.0 0.0) (`self.Patrol2`)
        (:`OnSuccess`
          (`KismetSystemLibrary.Delay` 5.0)
          (`self.Patrol`))))))

(event `Roam`
  (`|AIMoveTo` self (`NavigationSystem.GetRandomPointInNavigableRadius` (`self.K2_GetActorLocation`) 500.0)
    (:`OnSuccess`
      (`KismetSystemLibrary.Delay` (`KismetMathLibrary.RandomFloatInRange` 0.0 0.5))
      (`self.DecideState`))))

(event `ChasePlayer`
  (params (PlayerToChase :type "/Game/Player/ThirdPersonCharacter Object Reference"))
  (`|AIMoveTo` self (0.0 0.0 0.0) PlayerToChase 5.0
    (:`OnSuccess`
      (`self.OnPerformAttack`)
      (`KismetSystemLibrary.Delay` 5.0)
      (`self.DecideState`))))

(event `CustomEvent`
  (`|AIMoveTo` self (0.0 0.0 0.0) (`self.Patrol1`) 5.0
    (:`OnSuccess`
      (`KismetSystemLibrary.Delay` (`self.PatrolWait`))
      (`|AIMoveTo` self (0.0 0.0 0.0) (`self.Patrol2`)
        (:`OnSuccess`
          (`KismetSystemLibrary.Delay` (`self.PatrolWait`))
          (`self.DecideState`))))))

(event `self.PawnSensor.OnSeePawn`
  (params (Pawn :type "Pawn Object Reference"))
  ;[1 1 1] Chase player when we see them
  (if (not (`self.SeenPlayer`))
    (cast `/Game/Player/ThirdPersonCharacter` Pawn)))

(fn `DecideState`
  (cast `/Game/Player/ThirdPersonCharacter` (`GameplayStatics.GetPlayerCharacter` 0))
  (switch `/Game/AI_Data/EAIState` (`self.AIState`)
    (:`NewEnumerator3`
      (`self.Patrol`))))

(fn `UserConstructionScript`)
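; LavaLift is a one-shot interactable lift that the player activates with E or the gamepad left face button while overlapping its Sphere.
; Tick shows a keyboard or gamepad prompt based on the gameplay controller's input mode and yaws Middle with the camera until use.
; Activation disables the trigger, enables Box collision and plays a sound.
; The plate, light and furnace then rise a fixed step per frame, with no delta-time scaling or stop.
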(event `self.ReceiveTick`
  (params (DeltaSeconds :type "Float (single-precision)"))
  (bind _returnvalue (`GameplayStatics.GetPlayerController` 0))
  (bind _box (`self.Box`))
  (bind _returnvalue_2 (`PrimitiveComponent.IsOverlappingActor` (`self.Sphere`) (`GameplayStatics.GetPlayerPawn` 0)))
  (bind _asbp_gameplay_controller (cast `/Game/Blueprints/BP_GameplayController` (`GameplayStatics.GetPlayerController` 0)))
  (bind _usinggamepad (`/Game/Blueprints/BP_GameplayController.UsingGamepad` _asbp_gameplay_controller))
  (`SceneComponent.SetVisibility` (`self.Keyboard`) (and _returnvalue_2 (not _usinggamepad)) false)
  (`SceneComponent.SetVisibility` (`self.Gamepad`) (and _returnvalue_2 _usinggamepad) false)
  (if (`self.Used`)
    (`SceneComponent.K2_AddLocalOffset` (`self.Fire_Plate_Floor_1`) (0.0 0.0 1.0) false false)
    (`SceneComponent.K2_AddLocalOffset` (`self.PointLight`) (0.0 0.0 1.0) false false)
    (`SceneComponent.K2_AddLocalOffset` (`self.SM_Env_Fire_Furnace`) (0.0 0.0 1.0) false false)
    (else
      (`SceneComponent.K2_SetRelativeRotation` (`self.Middle`) (`KismetMathLibrary.MakeRotator` 0.0 0.0 (+ (.yaw (`PlayerCameraManager.GetCameraRotation` (`GameplayStatics.GetPlayerCameraManager` 0))) 90.0)) false false)
      (if (and _returnvalue_2 (not (`self.Used`)) (or (`PlayerController.WasInputKeyJustPressed` _returnvalue "E") (`PlayerController.WasInputKeyJustPressed` _returnvalue "Gamepad_FaceButton_Left")))
        (set `self.Used` true)
        (`PrimitiveComponent.SetCollisionResponseToAllChannels` (`self.Sphere`) "ECR_Ignore")
        (`GameplayStatics.SpawnSoundAttached` "/Game/Assignment/Sounds/lava_lift.lava_lift" (`self.SM_Env_Fire_Furnace`))
        (`PrimitiveComponent.SetCollisionObjectType` _box "ECC_WorldDynamic")
        (`PrimitiveComponent.SetCollisionEnabled` _box "QueryAndPhysics")))))

(fn `UserConstructionScript`)
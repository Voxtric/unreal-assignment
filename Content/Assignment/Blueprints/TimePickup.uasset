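; TimePickup is a collectible actor that grants the player extra time.
; On overlap with an AssignmentCharacter, it adds a fixed amount to the character's Time, clamps it to a maximum, plays a 2D pickup sound and destroys itself.
; Each tick it spins its static mesh around roll and yaw, scaled by delta time.
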(event `self.ReceiveActorBeginOverlap`
  (params (OtherActor :type "Actor Object Reference"))
  (bind _asassignment_character (cast `AssignmentCharacter` OtherActor))
  (bind _output_get (set `AssignmentCharacter.Time` (+ (`AssignmentCharacter.Time` _asassignment_character) 20.0) _asassignment_character))
  (if (> _output_get 600.0)
    (set `AssignmentCharacter.Time` 600.0 _asassignment_character))
  (`GameplayStatics.PlaySound2D` "/Game/Assignment/Sounds/time_pickup.time_pickup")
  (`self.K2_DestroyActor`))

(event `self.ReceiveTick`
  (params (DeltaSeconds :type "Float (single-precision)"))
  (bind _returnvalue (* DeltaSeconds 100.0))
  (`SceneComponent.K2_AddRelativeRotation` (`self.StaticMesh`) (`KismetMathLibrary.MakeRotator` _returnvalue 0.0 _returnvalue) false true))

(fn `UserConstructionScript`)
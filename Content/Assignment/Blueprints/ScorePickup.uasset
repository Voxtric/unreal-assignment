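; Score pickup actor that awards points to the player character on overlap.
; When an AssignmentCharacter overlaps it, the pickup adds a fixed amount to that character's Score, plays a 2D pickup sound and destroys itself.
; Each tick it spins its static mesh on the roll and yaw axes, scaled by delta time for a frame-rate independent rotation.
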(event `self.ReceiveActorBeginOverlap`
  (params (OtherActor :type "Actor Object Reference"))
  (bind _asassignment_character (cast `AssignmentCharacter` OtherActor))
  (set `AssignmentCharacter.Score` (+ (`AssignmentCharacter.Score` _asassignment_character) 15) _asassignment_character)
  (`GameplayStatics.PlaySound2D` "/Game/Assignment/Sounds/score_pickup.score_pickup")
  (`self.K2_DestroyActor`))

(event `self.ReceiveTick`
  (params (DeltaSeconds :type "Float (single-precision)"))
  (bind _returnvalue (* DeltaSeconds 100.0))
  (`SceneComponent.K2_AddRelativeRotation` (`self.StaticMesh`) (`KismetMathLibrary.MakeRotator` _returnvalue 0.0 _returnvalue) false true))

(fn `UserConstructionScript`)
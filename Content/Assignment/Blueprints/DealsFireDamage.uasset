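; Fire hazard actor that burns any ThirdPersonCharacter that begins overlapping it.
; Attaches a fire emitter to the character's mesh, reusing it while valid, and applies constant damage at a fixed delay while the overlap lasts.
; The loop ends when the overlap ends or TakeDamage returns true.
; It then applies up to three trailing hits as an afterburn, stopping early on a true return, and deactivates the emitter.
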(event `self.ReceiveActorBeginOverlap`
  (params (OtherActor :type "Actor Object Reference"))
  (bind _damageconstant (`self.DamageConstant`))
  (bind _damagefrequenceyconstant (`self.DamageFrequenceyConstant`))
  (bind _asthird_person_character (cast `/Game/Player/ThirdPersonCharacter` OtherActor))
  (if (`self.DealingDamage`)
    (set `self.DealingDamage` true))
  (`/Engine/EditorBlueprintResources/StandardMacros.IsValid` (stale _returnvalue)
    (:`Is Valid`
      _)
    (:`Is Not Valid`
      (bind _returnvalue (`GameplayStatics.SpawnEmitterAttached` "/Game/StarterContent/Particles/P_Fire.P_Fire" (`Character.Mesh` _asthird_person_character) "None" (0.0 0.0 100.0) (struct) "KeepRelativeOffset" false))))
  (`ActorComponent.Activate` _returnvalue true)
  (bind _died (`/Game/Player/ThirdPersonCharacter.TakeDamage` _asthird_person_character _damageconstant :!label _label))
  (`KismetSystemLibrary.Delay` _damagefrequenceyconstant)
  (if (and (not _died) (`self.IsOverlappingActor` OtherActor))
    (goto _label)
    (else
      (bind _died_2 (`/Game/Player/ThirdPersonCharacter.TakeDamage` _asthird_person_character _damageconstant))
      (if (not _died_2)
        (`KismetSystemLibrary.Delay` _damagefrequenceyconstant)
        (bind _died_3 (`/Game/Player/ThirdPersonCharacter.TakeDamage` _asthird_person_character _damageconstant))
        (if (not _died_3)
          (`KismetSystemLibrary.Delay` _damagefrequenceyconstant)
          (`/Game/Player/ThirdPersonCharacter.TakeDamage` _asthird_person_character _damageconstant)))
      (set `self.DealingDamage` false)
      (`ActorComponent.Deactivate` _returnvalue))))

(fn `UserConstructionScript`)
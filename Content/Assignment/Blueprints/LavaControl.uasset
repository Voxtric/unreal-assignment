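; LavaControl is a one-shot interactable gear that removes three lava components, which are lethal to the player.
; Tick pulses a light and shows prompt text inside the Sphere, where E or gamepad left face button starts a four-second spin with sound, destroys the lava and disables Sphere collision.
; Actor overlaps outside the Sphere zero ThirdPersonCharacter health, trigger its damage event and attach fire.
; Once spun, the light stays off.
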(event `self.ReceiveTick`
  (params (DeltaSeconds :type "Float (single-precision)"))
  (bind _returnvalue (`GameplayStatics.GetPlayerController` 0))
  (bind _returnvalue_2 (`PrimitiveComponent.IsOverlappingActor` (`self.Sphere`) (`GameplayStatics.GetPlayerPawn` 0)))
  (if (`self.Spun`)
    (`LightComponent.SetIntensity` (`self.PointLight`) 0.0)
    (else
      (`SceneComponent.SetVisibility` (`self.TextRender`) _returnvalue_2 false)
      (`LightComponent.SetIntensity` (`self.PointLight`) (* (`KismetMathLibrary.Abs` (`KismetMathLibrary.Sin` (* (`GameplayStatics.GetRealTimeSeconds`) 2.0))) 50.0))
      (if (`self.Spin`)
        (`self.K2_SetActorRotation` (`KismetMathLibrary.ComposeRotators` (`self.K2_GetActorRotation`) (`KismetMathLibrary.MakeRotator` 0.0 (* DeltaSeconds 100.0))))
        (elif (and _returnvalue_2 (not (`self.Spun`)) (or (`PlayerController.WasInputKeyJustPressed` _returnvalue "E") (`PlayerController.WasInputKeyJustPressed` _returnvalue "Gamepad_FaceButton_Left")))
          (bind _returnvalue_3 (`GameplayStatics.SpawnSoundAtLocation` "/Game/Assignment/Sounds/turning_gear.turning_gear" (`SceneComponent.K2_GetComponentLocation` (`self.PointLight`))))
          (set `self.Spin` true)
          (`ActorComponent.K2_DestroyComponent` (`self.Lava1`))
          (`ActorComponent.K2_DestroyComponent` (`self.Lava2`))
          (`ActorComponent.K2_DestroyComponent` (`self.Lava3`))
          (`PrimitiveComponent.SetCollisionResponseToAllChannels` (`self.Sphere`) "ECR_Ignore")
          (`KismetSystemLibrary.Delay` 4.0)
          (set `self.Spin` false)
          (set `self.Spun` true)
          (`AudioComponent.Stop` _returnvalue_3))))))

(event `self.ReceiveActorBeginOverlap`
  (params (OtherActor :type "Actor Object Reference"))
  (if (not (`PrimitiveComponent.IsOverlappingActor` (`self.Sphere`) OtherActor))
    (bind _asthird_person_character (cast `/Game/Player/ThirdPersonCharacter` OtherActor))
    (set `AssignmentCharacter.TotalHealth` 0.0 _asthird_person_character)
    (`/Game/Player/ThirdPersonCharacter.DamageTaken_Event` _asthird_person_character)
    (`GameplayStatics.SpawnEmitterAttached` "/Game/StarterContent/Particles/P_Fire.P_Fire" (`Character.Mesh` _asthird_person_character))))

(fn `UserConstructionScript`)
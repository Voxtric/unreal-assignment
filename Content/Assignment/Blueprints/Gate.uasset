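; Gate actor that rises when an actor overlaps it and lowers when the overlap ends.
; A timeline drives the static mesh up to a scaled Z offset from the world location cached in the construction script, reversing to close.
; GateRise plays from the start on opening and from a later time offset on closing, stopping when the timeline finishes.
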(event `self.ReceiveBeginPlay`
  (`AudioComponent.Stop` (`self.gate_rise`)))

(event `self.ReceiveActorBeginOverlap`
  (params (OtherActor :type "Actor Object Reference"))
  (bind _gate_rise (`self.gate_rise`))
  (`AudioComponent.Play` _gate_rise 0.0)
  (bind (_direction _dooropening) (`Timeline|GateTimeline` :!label _label)
    (:`Update`
      (`SceneComponent.K2_SetWorldLocation` (`self.StaticMesh`) (+ (`KismetMathLibrary.MakeVector` 0.0 0.0 (* _dooropening 200.0)) (`self.StartLocation`)) false false))
    (:`Finished`
      (`AudioComponent.Stop` _gate_rise))))

(event `self.ReceiveActorEndOverlap`
  (params (OtherActor :type "Actor Object Reference"))
  (`AudioComponent.Play` (`self.gate_rise`) 1.8)
  (goto _label :!via `Reverse`))

(fn `UserConstructionScript`
  (set `self.StartLocation` (`SceneComponent.K2_GetComponentLocation` (`self.StaticMesh`))))
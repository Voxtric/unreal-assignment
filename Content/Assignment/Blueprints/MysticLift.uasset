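; MysticLift is a platform actor that the Artifact powers up to become a spinning lift.
; Any actor overlap stops the first found Artifact following the player, and Tick lerps its sphere and light toward the Trigger.
; On arrival the Artifact's sphere and light hide, the lift's lights and mesh appear, and it becomes active.
; While active, the platform rises and yaws each frame as long as it overlaps the Light component.
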(event `self.ReceiveTick`
  (params (DeltaSeconds :type "Float (single-precision)"))
  (bind _sm_fire_fort_penta_plat_2 (`self.SM_Fire_Fort_Penta_Plat_2`))
  (bind _returnvalue (`SceneComponent.K2_GetComponentLocation` (`self.Trigger`)))
  (if (`self.BecomeLift`)
    (bind _outactors (`GameplayStatics.GetAllActorsOfClass` "/Game/Assignment/Blueprints/Artifact.Artifact_C"))
    (bind _item (`KismetArrayLibrary.Array_Get` _outactors))
    (bind _sphere (`/Game/Assignment/Blueprints/Artifact.Sphere` _item))
    (bind _returnvalue_2 (`SceneComponent.K2_GetComponentLocation` _sphere))
    (bind _returnvalue_3 (`KismetMathLibrary.VLerp` _returnvalue_2 _returnvalue 0.02))
    (`SceneComponent.K2_SetWorldLocation` _sphere _returnvalue_3 false true)
    (bind _pointlight (`/Game/Assignment/Blueprints/Artifact.PointLight` _item))
    (`SceneComponent.K2_SetWorldLocation` _pointlight _returnvalue_3 false true)
    (if (< (`KismetMathLibrary.Abs` (`KismetMathLibrary.VSize` (- _returnvalue _returnvalue_2))) 1.0)
      (`SceneComponent.SetVisibility` (`self.Light`) true false)
      (`SceneComponent.SetVisibility` (`self.StaticMesh1`) true false)
      (`SceneComponent.SetVisibility` (`self.PointLight`) true false)
      (`SceneComponent.SetVisibility` (`self.PointLight1`) true false)
      (`SceneComponent.SetVisibility` (`self.PointLight2`) true false)
      (`SceneComponent.SetVisibility` (`self.PointLight3`) true false)
      (`SceneComponent.SetVisibility` (`self.PointLight4`) true false)
      (`SceneComponent.SetVisibility` (`self.PointLight5`) true false)
      (`SceneComponent.SetVisibility` (`self.PointLight6`) true false)
      (`SceneComponent.SetVisibility` (`self.PointLight7`) true false)
      (set `self.Active` true)
      (set `self.BecomeLift` false)
      (`SceneComponent.SetVisibility` _sphere false false)
      (`SceneComponent.SetVisibility` _pointlight false false))
    (elif (and (`PrimitiveComponent.IsOverlappingComponent` (`self.SM_Fire_Fort_Penta_Plat_2`) (`self.Light`)) (`self.Active`))
      (`SceneComponent.K2_AddRelativeLocation` _sm_fire_fort_penta_plat_2 (`KismetMathLibrary.MakeVector` 0.0 0.0 (* DeltaSeconds 200.0)) false false)
      (`SceneComponent.K2_AddRelativeRotation` _sm_fire_fort_penta_plat_2 (`KismetMathLibrary.MakeRotator` 0.0 0.0 (* DeltaSeconds 70.0)) false false))))

(event `self.ReceiveActorBeginOverlap`
  (params (OtherActor :type "Actor Object Reference"))
  (bind _outactors (`GameplayStatics.GetAllActorsOfClass` "/Game/Assignment/Blueprints/Artifact.Artifact_C"))
  (set `/Game/Assignment/Blueprints/Artifact.FollowPlayer` false (`KismetArrayLibrary.Array_Get` _outactors))
  (set `self.BecomeLift` true))

(fn `UserConstructionScript`)
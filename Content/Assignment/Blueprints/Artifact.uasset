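; Artifact actor that bobs in place until the player activates it, then breaks free and follows the player as a glowing light.
; Tick shows a text prompt while the player overlaps the trigger and polls E or gamepad face-left for activation.
; Activation widens the light, swaps collision, then after a delay shatters four destructibles, brightens the sphere's material and plays a breaking sound.
; A FollowPlayer flag switches sine bobbing to lerped trailing beside the pawn.
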(event `self.ReceiveTick`
  (params (DeltaSeconds :type "Float (single-precision)"))
  (bind _returnvalue (`GameplayStatics.GetPlayerController` 0))
  (bind _returnvalue_2 (`GameplayStatics.GetPlayerPawn` 0))
  (bind _returnvalue_3 (`self.K2_GetActorLocation`))
  (bind _box (`self.Box`))
  (bind _returnvalue_4 (`PrimitiveComponent.IsOverlappingActor` (`self.Trigger`) (`GameplayStatics.GetPlayerPawn` 0)))
  (bind _returnvalue_5 (`KismetMathLibrary.MakeVector` 0.0 0.0 (* (`KismetMathLibrary.Sin` (`KismetSystemLibrary.GetGameTimeInSeconds`)) DeltaSeconds 15.0)))
  (bind _returnvalue_6 (`KismetMathLibrary.VLerp` (`SceneComponent.K2_GetComponentLocation` (`self.PointLight`)) (+ (`self.K2_GetActorLocation` _returnvalue_2) (* (+ (`self.GetActorRightVector` _returnvalue_2) (`self.GetActorUpVector` _returnvalue_2)) 75.0)) (* DeltaSeconds 3.0)))
  (`SceneComponent.SetVisibility` (`self.TextRender`) _returnvalue_4 false)
  (if (`self.FollowPlayer`)
    (`SceneComponent.K2_SetWorldLocation` (`self.PointLight`) _returnvalue_6 false true)
    (`SceneComponent.K2_SetWorldLocation` (`self.Sphere`) _returnvalue_6 false true)
    (else
      (`SceneComponent.K2_AddLocalOffset` (`self.Sphere`) _returnvalue_5 false false)
      (`SceneComponent.K2_AddLocalOffset` (`self.PointLight`) _returnvalue_5 false false)
      (if (and _returnvalue_4 (or (`PlayerController.WasInputKeyJustPressed` _returnvalue "E") (`PlayerController.WasInputKeyJustPressed` _returnvalue "Gamepad_FaceButton_Left")))
        (`PointLightComponent.SetAttenuationRadius` (`self.PointLight`) 3000.0)
        (`PrimitiveComponent.SetCollisionResponseToAllChannels` (`self.Trigger`) "ECR_Ignore")
        (`PrimitiveComponent.SetCollisionObjectType` _box "ECC_WorldDynamic")
        (`PrimitiveComponent.SetCollisionEnabled` _box "QueryAndPhysics")
        (`KismetSystemLibrary.Delay` 3.0)
        (`DestructibleComponent.ApplyRadiusDamage` (`self.Destructible`) 100.0 _returnvalue_3 100.0 100.0 true)
        (`DestructibleComponent.ApplyRadiusDamage` (`self.Destructible1`) 100.0 _returnvalue_3 100.0 100.0 true)
        (`DestructibleComponent.ApplyRadiusDamage` (`self.Destructible2`) 100.0 _returnvalue_3 100.0 100.0 true)
        (`DestructibleComponent.ApplyRadiusDamage` (`self.Destructible3`) 100.0 _returnvalue_3 100.0 100.0 true)
        (set `self.FollowPlayer` true)
        (bind _returnvalue_7 (`KismetMaterialLibrary.CreateDynamicMaterialInstance` "/Game/Assignment/Materials/Artifact.Artifact"))
        (`MaterialInstanceDynamic.SetScalarParameterValue` _returnvalue_7 "Intensity" 1.0)
        (`PrimitiveComponent.SetMaterial` (`self.Sphere`) 0 _returnvalue_7)
        (bind _returnvalue_8 (`GameplayStatics.SpawnSoundAtLocation` "/Game/Assignment/Sounds/breaking_stone.breaking_stone" _returnvalue_3))
        (`AudioComponent.FadeOut` _returnvalue_8 2.0 0.0)))))

(fn `UserConstructionScript`)
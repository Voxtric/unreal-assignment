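; Fire damage trigger that sets an overlapping actor of the cast type alight with an attached P_Fire emitter and damages it over time.
; It repeats TakeDamage on a delay while the overlap lasts and the call returns false.
; Afterwards it applies up to three trailing damage ticks, deactivating the reusable emitter only if all three return false.
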(event `self.ReceiveActorBeginOverlap`
  (params (OtherActor :type "Actor Object Reference"))
  (bind _damageconstant (`self.DamageConstant`))
  (bind _damagefrequenceyconstant (`self.DamageFrequenceyConstant`))
  (cast `` OtherActor)
  (`/Engine/EditorBlueprintResources/StandardMacros.IsValid` (stale _returnvalue)
    (:`Is Valid`
      _)
    (:`Is Not Valid`
      (bind _returnvalue (`GameplayStatics.SpawnEmitterAttached` "/Game/StarterContent/Particles/P_Fire.P_Fire" (`Character.Mesh`) "None" (0.0 0.0 100.0) (struct) "KeepRelativeOffset" false))))
  (`ActorComponent.Activate` _returnvalue true)
  (bind _died (`self.TakeDamage` _damageconstant :!label _label))
  (`KismetSystemLibrary.Delay` _damagefrequenceyconstant)
  (if (and (not _died) (`self.IsOverlappingActor` OtherActor))
    (goto _label)
    (else
      (bind _died_2 (`self.TakeDamage` _damageconstant))
      (if (not _died_2)
        (`KismetSystemLibrary.Delay` _damagefrequenceyconstant)
        (bind _died_3 (`self.TakeDamage` _damageconstant))
        (if (not _died_3)
          (`KismetSystemLibrary.Delay` _damagefrequenceyconstant)
          (bind _died_4 (`self.TakeDamage` _damageconstant))
          (if (not _died_4)
            (`ActorComponent.Deactivate` _returnvalue)))))))

(fn `UserConstructionScript`)
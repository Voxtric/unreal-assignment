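; A one-shot trigger that plays the minecart chase set piece when an actor overlaps it.
; It plays the CartChase level sequence with an attenuated minecart sound attached to the cart mesh.
; After a fixed delay it stops both, turns on physics for the cart, launches it with a strong force and destroys the MinecartHit actor.
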(event `self.ReceiveActorBeginOverlap`
  (params (OtherActor :type "Actor Object Reference"))
  (bind _staticmeshcomponent (`StaticMeshActor.StaticMeshComponent` (`self.Minecart`)))
  (if (not (`self.Played`))
    (set `self.Played` true)
    (bind _returnvalue (`LevelSequencePlayer.CreateLevelSequencePlayer` "/Game/Assignment/Sequences/CartChase.CartChase"))
    (bind _output_get (set `self.NewVar_0` _returnvalue))
    (`LevelSequencePlayer.Play` _returnvalue)
    (`LevelSequencePlayer.Play` _output_get)
    (bind _returnvalue_2 (`GameplayStatics.SpawnSoundAttached` "/Game/Assignment/Sounds/minecart.minecart" _staticmeshcomponent "None" (0.0 0.0 0.0) (struct) "KeepRelativeOffset" false 0.25 1.0 0.0 "/Game/Assignment/Sounds/MinecartAttenuation.MinecartAttenuation"))
    (`KismetSystemLibrary.Delay` 7.8)
    (`LevelSequencePlayer.Stop` _output_get)
    (`PrimitiveComponent.SetSimulatePhysics` _staticmeshcomponent true)
    (`PrimitiveComponent.AddForce` _staticmeshcomponent (20000.0 -100000.0 0.0) "None" true)
    (`AudioComponent.Stop` _returnvalue_2)
    (`self.K2_DestroyActor` (`self.MinecartHit`))))

(fn `UserConstructionScript`)
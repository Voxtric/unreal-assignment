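; EndGame is a trigger Blueprint that runs the end-of-game transition when any actor begins overlapping it.
; It spawns a level sequence actor to play the FadeOut sequence, then after a five-second delay adds the Loading widget to the viewport.
; A brief delay later it casts the player character to ThirdPersonCharacter and calls its EndGame function.
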(event `self.ReceiveActorBeginOverlap`
  (params (OtherActor :type "Actor Object Reference"))
  (bind _returnvalue (`|SpawnActorFromClass` "/Script/LevelSequence.LevelSequenceActor" (`KismetMathLibrary.MakeTransform` (0.0 0.0 0.0)) "Undefined" "OverrideRootScale"))
  (`LevelSequenceActor.SetSequence` _returnvalue "/Game/Assignment/Sequences/FadeOut.FadeOut")
  (`LevelSequencePlayer.Play` (`LevelSequenceActor.SequencePlayer` _returnvalue))
  (`KismetSystemLibrary.Delay` 5.0)
  (bind _returnvalue_2 (`|CreateWidget` "/Game/UI/Loading.Loading_C" (`GameplayStatics.GetPlayerController` 0)))
  (`UserWidget.AddToViewport` _returnvalue_2 1)
  (`KismetSystemLibrary.Delay` 0.01)
  (bind _asthird_person_character (cast `/Game/Player/ThirdPersonCharacter` (`GameplayStatics.GetPlayerCharacter` 0)))
  (`/Game/Player/ThirdPersonCharacter.EndGame` _asthird_person_character false))

(fn `UserConstructionScript`)
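; EndGame is an overlap-triggered actor that sends the player to the high score screen when their score qualifies.
; On overlap, it loads saved scores through the GameplayController and compares the overlapping AssignmentCharacter's Score to the tenth entry.
; A higher score is saved through the character's SaveValue and opens the HighScores level; otherwise nothing happens.
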(event `self.ReceiveActorBeginOverlap`
  (params (OtherActor :type "Actor Object Reference"))
  (bind _asgameplay_controller (cast `GameplayController` (`GameplayStatics.GetPlayerController` 0)))
  (bind _returnvalue (`GameplayController.LoadScoreValues` _asgameplay_controller))
  (bind _asassignment_character (cast `AssignmentCharacter` OtherActor))
  (bind _score (`AssignmentCharacter.Score` _asassignment_character))
  (if (> _score (`KismetArrayLibrary.Array_Get` _returnvalue 9))
    (`AssignmentCharacter.SaveValue` _asassignment_character "Score" (`KismetMathLibrary.Conv_IntToDouble` _score))
    (`GameplayStatics.OpenLevel` "HighScores")))

(fn `UserConstructionScript`)
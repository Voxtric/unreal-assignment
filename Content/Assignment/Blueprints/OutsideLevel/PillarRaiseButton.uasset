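; A pressure button that raises a target pillar when the player steps on its trigger, then lowers it again after DownTime.
; The overlap sinks the button and lifts the pillar, and a delay later both return.
; Separate timelines drive each move, offsetting from the location captured as that move starts.
; A Ready flag blocks retriggering until the pillar finishes lowering.
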(event `self.trigger.OnComponentBeginOverlap`
  (params (OverlappedComponent :type "PrimitiveComponent Object Reference") (OtherActor :type "Actor Object Reference") (OtherComp :type "PrimitiveComponent Object Reference") (OtherBodyIndex :type Integer) (bFromSweep :type Boolean) (SweepResult :type "HitResult Structure (by ref)"))
  ;[1 1 1] Trigger Events
  (if (and (== (`GameplayStatics.GetPlayerCharacter` 0) OtherActor) (`self.ready`))
    (set `self.ready` false)
    (`self.buttonLower`)
    (`self.pillarRaise`)
    (`KismetSystemLibrary.Delay` (`self.downTime`))
    (`self.buttonRaise`)
    (`self.pillarLower`)))

(event `pillarRaise`
  ;[1 1 1] Move the pillar
  (set `self.initialPillarLocation` (`self.K2_GetActorLocation` (`self.targetPillar`)))
  (bind (_direction _movement) (`Timeline|pillarMovement` :!via `PlayFromStart`)
    (:`Update`
      (`self.K2_SetActorLocation` (`self.targetPillar`) (+ (* _movement 2000) (`self.initialPillarLocation`)) false false))))

(event `pillarLower`
  ;[1 1 1] Move the pillar
  (set `self.initialPillarLocation` (`self.K2_GetActorLocation` (`self.targetPillar`)))
  (bind (_direction _movement) (`Timeline|pillarMovement2` :!via `PlayFromStart`)
    (:`Update`
      (`self.K2_SetActorLocation` (`self.targetPillar`) (+ (`self.initialPillarLocation`) (* _movement -2000)) false false))
    (:`Finished`
      (set `self.ready` true))))

(event `buttonLower`
  ;[1 1 1] MoveButton
  (set `self.initialButtonLocation` (`SceneComponent.K2_GetComponentLocation` (`self.button`)))
  (bind (_direction _movement) (`Timeline|buttonMove` :!via `PlayFromStart`)
    (:`Update`
      (`SceneComponent.K2_SetWorldLocation` (`self.button`) (+ (* _movement -20) (`self.initialButtonLocation`)) false false))))

(event `buttonRaise`
  ;[1 1 1] MoveButton
  (set `self.initialButtonLocation` (`SceneComponent.K2_GetComponentLocation` (`self.button`)))
  (bind (_direction _movement) (`Timeline|buttonMove2` :!via `PlayFromStart`)
    (:`Update`
      (`SceneComponent.K2_SetWorldLocation` (`self.button`) (+ (`self.initialButtonLocation`) (* _movement 20)) false false))))

(fn `UserConstructionScript`)
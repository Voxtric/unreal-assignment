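; An outside-level fire statue that passes its flame to the bridge gate when the player enters its collision sphere.
; On overlap it casts its gate reference to the bridge gate and calls LightFire with its torch index.
; It then deactivates the statue fire and runs a timeline that scales the fire light's intensity, deactivating the light when the timeline finishes.
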(event `self.collisionSphere.OnComponentBeginOverlap`
  (params (OverlappedComponent :type "PrimitiveComponent Object Reference") (OtherActor :type "Actor Object Reference") (OtherComp :type "PrimitiveComponent Object Reference") (OtherBodyIndex :type Integer) (bFromSweep :type Boolean) (SweepResult :type "HitResult Structure (by ref)"))
  (bind _firelight (`self.fireLight`))
  (if (== OtherActor (`GameplayStatics.GetPlayerCharacter` 0))
    (bind _asoutside_level_bridge_gate (cast `/Game/Assignment/Blueprints/OutsideLevel/OutsideLevel_BridgeGate` (`self.theGate`)))
    (`/Game/Assignment/Blueprints/OutsideLevel/OutsideLevel_BridgeGate.lightFire` _asoutside_level_bridge_gate (`self.torchIndex`))
    (`ActorComponent.Deactivate` (`self.statueFire`))
    (bind (_direction _intensity) (`Timeline|light fade`)
      (:`Update`
        (`LightComponent.SetIntensity` _firelight (* 5000 _intensity)))
      (:`Finished`
        (`ActorComponent.Deactivate` _firelight)))))

(fn `UserConstructionScript`)
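; Bridge gate in the outside level that lowers once its left, right and centre fires are all lit.
; LightFire activates the indexed fire with a sound, sets its flag and calls FireLit to check all three.
; When all are lit, a cutscene plays and, after a short delay, a timeline slides the gate down while move input is ignored.
; The first fire lit also plays that same gate-opening sequence.
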(event `fireLit`
  (bind _returnvalue (`GameplayStatics.GetPlayerController` 0))
  (set `self.numFiresLit` (+ (`self.numFiresLit`) 1))
  (if (and (`self.leftFireLit`) (`self.rightFireLit`) (`self.centreFireLit`) (not (`self.gateLowered`)))
    (`Controller.SetIgnoreMoveInput` _returnvalue true)
    (bind _returnvalue_2 (`LevelSequencePlayer.CreateLevelSequencePlayer` "/Game/Assignment/Sequences/OutsideLevel_GateOpenSequence.OutsideLevel_GateOpenSequence"))
    (`LevelSequencePlayer.Play` _returnvalue_2)
    (`KismetSystemLibrary.Delay` 0.7)
    (bind (_direction _movement) (`Timeline|gateMoveDown` :!via `PlayFromStart`)
      (:`Update`
        (`SceneComponent.K2_SetWorldLocation` (`self.gate`) (+ (* _movement -700) (`self.StartLocation`)) false false))
      (:`Finished`
        (set `self.gateLowered` true)
        (`Controller.ResetIgnoreMoveInput` _returnvalue)))))

(fn `lightFire`
  (params (fireIndex :type Integer))
  (bind _returnvalue (`GameplayStatics.GetPlayerController` 0))
  (bind _leftfire (`self.leftFire`))
  (bind _centrefire (`self.centreFire`))
  (bind _rightfire (`self.rightFire`))
  (if (== (`self.numFiresLit`) 0)
    ;[1 1 1] Play cutscene on first fire
    (`Controller.SetIgnoreMoveInput` _returnvalue true)
    (bind _returnvalue_2 (`LevelSequencePlayer.CreateLevelSequencePlayer` "/Game/Assignment/Sequences/OutsideLevel_GateOpenSequence.OutsideLevel_GateOpenSequence"))
    (`LevelSequencePlayer.Play` _returnvalue_2)
    (`LevelSequencePlayer.SetPlaybackPosition` _returnvalue_2 0.0) ; This needs to be done because the same cutscene will be used for watching the opening of the gate
    (`Controller.SetIgnoreMoveInput` _returnvalue false))
  (switch `int` fireIndex
    (:`0`
      ;[1 1 1] Put out the fires
      (`ActorComponent.Activate` _leftfire false)
      (`GameplayStatics.PlaySoundAtLocation` "/Game/StarterContent/Audio/Fire01_Cue.Fire01_Cue" (`SceneComponent.K2_GetComponentLocation` _leftfire) (struct) 1.0 1.0 0.0 "/Game/Blueprints/Animation/EnemyAt.EnemyAt")
      (set `self.leftFireLit` true))
    (:`1`
      (`ActorComponent.Activate` _rightfire false)
      (`GameplayStatics.PlaySoundAtLocation` "/Game/StarterContent/Audio/Fire01_Cue.Fire01_Cue" (`SceneComponent.K2_GetComponentLocation` _rightfire) (struct) 1.0 1.0 0.0 "/Game/Blueprints/Animation/EnemyAt.EnemyAt")
      (set `self.rightFireLit` true))
    (:`2`
      (`ActorComponent.Activate` _centrefire false)
      (`GameplayStatics.PlaySoundAtLocation` "/Game/StarterContent/Audio/Fire01_Cue.Fire01_Cue" (`SceneComponent.K2_GetComponentLocation` _centrefire) (struct) 1.0 1.0 0.0 "/Game/Blueprints/Animation/EnemyAt.EnemyAt")
      (set `self.centreFireLit` true)))
  (`self.fireLit`))

(fn `UserConstructionScript`
  (set `self.StartLocation` (`SceneComponent.K2_GetComponentLocation` (`self.gate`))))
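; Explosive is a pickup actor that the player carries and that blows up on contact with a destructible actor.
; Any overlap sets PickedUp, after which Tick teleports the mesh each frame to a point in front of player character 0.
; Overlapping a DestructibleActor spawns an explosion effect and sound, applies radius damage with impulse to its destructible component, then destroys the explosive.
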(event `self.ReceiveActorBeginOverlap`
  (params (OtherActor :type "Actor Object Reference"))
  (bind _returnvalue (`SceneComponent.K2_GetComponentLocation` (`self.StaticMesh`)))
  (bind _returnvalue_2 (+ _returnvalue (0.0 0.0 50.0)))
  (set `self.PickedUp` true)
  (bind _asdestructible_actor (cast `DestructibleActor` OtherActor))
  (`GameplayStatics.SpawnEmitterAtLocation` "/Game/StarterContent/Particles/P_Explosion.P_Explosion" _returnvalue)
  (`DestructibleComponent.ApplyRadiusDamage` (`DestructibleActor.DestructibleComponent` _asdestructible_actor) 100.0 _returnvalue_2 100.0 100.0 true)
  (`GameplayStatics.PlaySoundAtLocation` "/Game/StarterContent/Audio/Explosion02.Explosion02" _returnvalue_2)
  (`self.K2_DestroyActor`))

(event `self.ReceiveTick`
  (params (DeltaSeconds :type "Float (single-precision)"))
  (bind _returnvalue (`GameplayStatics.GetPlayerCharacter` 0))
  (if (`self.PickedUp`)
    (`SceneComponent.K2_SetWorldLocation` (`self.StaticMesh`) (+ (`self.K2_GetActorLocation` _returnvalue) (* (`SceneComponent.GetForwardVector` (`Character.CapsuleComponent` _returnvalue)) 125)) false true)))

(fn `UserConstructionScript`)
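; Lift actor that descends with a sinusoidal sway while CanMove is set, then stops on overlapping StopTrigger and can start an intro cutscene.
; If the player is nearby, it spawns a sequence actor for IntoCutscene, blends to the camera named "Cutscene Camera" and disables character movement.
; View and walking return after a fixed delay, or earlier when Tick detects a Space or gamepad skip during playback.
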(event `self.ReceiveTick`
  (params (DeltaSeconds :type "Float (single-precision)"))
  (bind _returnvalue (`GameplayStatics.GetPlayerController` 0))
  (bind _returnvalue_2 (`KismetSystemLibrary.GetGameTimeInSeconds`))
  (`/Engine/EditorBlueprintResources/StandardMacros.IsValid` (stale `self.ReceiveActorBeginOverlap` _returnvalue_2)
    (:`Is Valid`
      (bind _sequenceplayer (`LevelSequenceActor.SequencePlayer` (stale `self.ReceiveActorBeginOverlap` _returnvalue_2)))
      (if (and (or (`PlayerController.WasInputKeyJustPressed` _returnvalue "SpaceBar") (`PlayerController.WasInputKeyJustPressed` _returnvalue "Gamepad_FaceButton_Bottom")) (`LevelSequencePlayer.IsPlaying` _sequenceplayer))
        (`LevelSequencePlayer.Stop` _sequenceplayer)
        (bind _asthird_person_character (cast `/Game/Player/ThirdPersonCharacter` (`GameplayStatics.GetPlayerCharacter` 0)))
        (`PlayerController.SetViewTargetWithBlend` (`GameplayStatics.GetPlayerController` 0) _asthird_person_character 0.0 "VTBlend_Linear" 0.0 false)
        (`CharacterMovementComponent.SetMovementMode` (`Character.CharacterMovement` _asthird_person_character) "MOVE_Walking" 0)))
    (:`Is Not Valid`
      _))
  (if (`self.CanMove`)
    (`self.K2_SetActorLocation` (+ (`self.K2_GetActorLocation`) (* (0.0 0.0 -100.0) DeltaSeconds) (* (40.0 40.0 80.0) (* DeltaSeconds (`KismetMathLibrary.DegCos` _returnvalue_2) (`KismetMathLibrary.Sin` _returnvalue_2)))))))

(event `self.ReceiveActorBeginOverlap`
  (params (OtherActor :type "Actor Object Reference"))
  (bind _returnvalue (`GameplayStatics.GetPlayerController` 0))
  (if (== OtherActor (`self.StopTrigger`))
    (set `self.CanMove` false)
    (if (< (`KismetMathLibrary.Abs` (`KismetMathLibrary.VSize` (- (`self.K2_GetActorLocation` (`GameplayStatics.GetPlayerPawn` 0)) (`self.K2_GetActorLocation`)))) 500.0)
      (bind _returnvalue_2 (`|SpawnActorFromClass` "/Script/LevelSequence.LevelSequenceActor" (`KismetMathLibrary.Conv_VectorToTransform` (`KismetMathLibrary.MakeVector` 0.0)) "AlwaysSpawn" "OverrideRootScale"))
      (`LevelSequenceActor.SetSequence` _returnvalue_2 "/Game/Assignment/Sequences/IntoCutscene.IntoCutscene")
      (`LevelSequencePlayer.Play` (`LevelSequenceActor.SequencePlayer` _returnvalue_2))
      (bind _outactors (`GameplayStatics.GetAllActorsOfClass` "/Script/Engine.CameraActor"))
      (bind _asthird_person_character (cast `/Game/Player/ThirdPersonCharacter` (`GameplayStatics.GetPlayerPawn` 0)))
      (for _array_element _outactors
        (if (`KismetStringLibrary.EqualEqual_StrStr` (`KismetSystemLibrary.GetDisplayName` _array_element) "Cutscene Camera")
          (`PlayerController.SetViewTargetWithBlend` _returnvalue _array_element 2.0 "VTBlend_EaseInOut" 1.0 false)
          (bind _charactermovement (`Character.CharacterMovement` _asthird_person_character))
          (`CharacterMovementComponent.SetMovementMode` _charactermovement "MOVE_None" 0)
          (break)))
      (`KismetSystemLibrary.Delay` 27.0)
      (`PlayerController.SetViewTargetWithBlend` _returnvalue _asthird_person_character 0.0 "VTBlend_Linear" 0.0 false)
      (`CharacterMovementComponent.SetMovementMode` _charactermovement "MOVE_Walking" 0))))

(fn `UserConstructionScript`)